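; Gameplay game mode that manages the connection to the GameSparks online service through its GameSparks component.
; BeginPlay disconnects and then reconnects using an API key and secret hard-coded in the graph.
; EndPlay disconnects for any reason other than a level transition.
; The availability delegate is bound but empty, and the debug prints for availability are never executed.
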(event OnGameSparksAvailableDelegate(GameSparks)
  (params (available :type Boolean))
  ;[1 0.3532 0 0] GameSparks
  ;;[0 0.4212 1] Receives feedback everytime connect and disconnect functions are called on GS component
)

(event EventEndPlay
  (params (EndPlayReason :type EEndPlayReason%20Enum :default "Destroyed"))
  ;[1 0.3532 0 0] GameSparks
  ;;[0 0.4212 1] Discconects the module via GS component then connects it - If our game shuts down for any reason that's not level transition GS module will disconnect
  (if (Utilities|Enum|NotEqual(Enum) (Utilities|Enum|LiteralenumEEndPlayReason EndPlayReason) "LevelTransition")
    (Class|GameSparksComponent|Disconnect (Variables|Default|GetGameSparks))))

(event EventBeginPlay
  (bind _gamesparks (Variables|Default|GetGameSparks))
  ;[1 0.3532 0 0] GameSparks
  ;;[0 0.4212 1] Discconects the module via GS component then connects it - If our game shuts down for any reason that's not level transition GS module will disconnect
  (Class|GameSparksComponent|Disconnect _gamesparks)
  (Class|GameSparksComponent|Connect _gamesparks "293711ZXWjA9" "DgnYnPUE2D0RetwKAy5XPUxxxN7pl36e" true false))

(fn ConstructionScript)