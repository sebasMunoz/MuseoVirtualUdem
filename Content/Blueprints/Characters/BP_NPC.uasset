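; BP_NPC is a non-player character with a selectable male or female appearance and a message for the player.
; On BeginPlay, SetNPCAvatar uses AvatarID to swap the skeletal mesh and its matching animation Blueprint class.
; ShowMessage casts player character 0 to ThirdPersonCharacter and writes this NPC's Message into its NPCMessageOnPlayer variable; nothing in this Blueprint calls it.
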(event EventBeginPlay
  (NPC|SetNPCAvatar (Variables|NPC|GetAvatarID)))

(event Collision|EventActorBeginOverlap
  (params (OtherActor :type Actor%20Object%20Reference)))

(event EventTick
  (params (DeltaSeconds :type Float%20%28single-precision%29)))

(fn ConstructionScript)

(fn ShowMessage
  ;[0 0.06667 1] Returna el mensaje del NPC
  (bind _asthird_person_character (Utilities|Casting|CastToThirdPersonCharacter (Game|GetPlayerCharacter 0)))
  (Variables|/Game/Blueprints/Characters/ThirdPersonCharacter.ThirdPersonCharacter_C|SetNPCMessageOnPlayer _asthird_person_character (Variables|NPC|Getmessage)))

(fn SetNPCAvatar
  (params (AvatarID :type Integer))
  (bind _skeletalmesh (Variables|Default|GetSkeletalMesh))
  (switch int AvatarID
    (:0
      (Class|SkinnedMeshComponent|SetSkeletalMesh _skeletalmesh "/Game/3DModels/NPC´s/NPC01/NPCMenMesh.NPCMenMesh" true)
      (Components|SkeletalMesh|SetAnimInstanceClass _skeletalmesh "/Game/3DModels/NPC´s/NPC01/Animations/BP_NPCMenAnimation.BP_NPCMenAnimation_C"))
    (:1
      (Class|SkinnedMeshComponent|SetSkeletalMesh _skeletalmesh "/Game/3DModels/NPC´s/NPC02/NPCWomanMesh.NPCWomanMesh" true)
      (Components|SkeletalMesh|SetAnimInstanceClass _skeletalmesh "/Game/3DModels/NPC´s/NPC02/Animations/BP_NPCWomanAnimation.BP_NPCWomanAnimation_C"))))