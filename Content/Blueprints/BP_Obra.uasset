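; BP_Obra is an interactable artwork actor holding metadata such as title, author, technique and origin.
; Interaction casts the player to ThirdPersonCharacter, writes a Spanish "press F" prompt with the title, sets its own Interactable flag, and copies the metadata onto the character.
; ShowInfo only prints the title, and EnableWidget returns ArtWorkUI.
; The event graph is empty, so these functions contain all the logic and none are called here.
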(event EventBeginPlay)

(event Collision|EventActorBeginOverlap
  (params (OtherActor :type Actor%20Object%20Reference)))

(event EventTick
  (params (DeltaSeconds :type Float%20%28single-precision%29)))

(fn ConstructionScript)

(fn Interaction
  (bind _asthird_person_character (Utilities|Casting|CastToThirdPersonCharacter (Game|GetPlayerCharacter 0)))
  (Variables|/Game/Blueprints/ThirdPersonCharacter.ThirdPersonCharacter_C|SetInteractionMessage _asthird_person_character (Utilities|String|Append "Presiona \"F\" para interactuar con: " (Variables|Obra|GetTitle)))
  (Variables|Obra|SetInteractable true)
  (Utilities|FlowControl|Sequence
    (:then_0
      (Variables|/Game/Blueprints/ThirdPersonCharacter.ThirdPersonCharacter_C|SetAuthor _asthird_person_character (Variables|Obra|GetAuthor)))
    (:then_1
      (Variables|/Game/Blueprints/ThirdPersonCharacter.ThirdPersonCharacter_C|SetTitle _asthird_person_character (Variables|Obra|GetTitle)))
    (:then_2
      (Variables|/Game/Blueprints/ThirdPersonCharacter.ThirdPersonCharacter_C|SetDateTime _asthird_person_character (Variables|Obra|GetDateTime)))
    (:then_3
      (Variables|/Game/Blueprints/ThirdPersonCharacter.ThirdPersonCharacter_C|SetTechnique _asthird_person_character (Variables|Obra|GetTechnique)))
    (:then_4
      (Variables|/Game/Blueprints/ThirdPersonCharacter.ThirdPersonCharacter_C|SetOrigin _asthird_person_character (Variables|Obra|GetOrigin)))
    (:then_5
      (Variables|/Game/Blueprints/ThirdPersonCharacter.ThirdPersonCharacter_C|SetDescription _asthird_person_character (Variables|Obra|GetDescription)))))

(fn ShowInfo
  (Development|PrintString (Utilities|String|Append "Interactuando con: " (Variables|Obra|GetTitle))))

(fn EnableWidget
  (return (Variables|Obra|GetArtWorkUI)))